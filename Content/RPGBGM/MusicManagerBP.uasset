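; Music manager that switches the level's background music between tracks in TrackList with a sequential fade.
; BeginPlay starts every track at once as muted 2D sounds, then raises the starting index to full volume.
; ChangeMusicTo sets the target index, and looping function timers fade the current track out, then the new one in.
; Requesting the track that is already current switches to the preceding index instead.
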(event `self.ReceiveBeginPlay`
  (for _array_element (`self.TrackList`)
    (bind _returnvalue (`GameplayStatics.CreateSound2D` _array_element 1.0 1.0 0.0 null))
    (`KismetArrayLibrary.Array_Add` (`self.musicreferences`) _returnvalue)
    (`AudioComponent.SetVolumeMultiplier` _returnvalue 0.0)
    (`AudioComponent.Play` _returnvalue 0.0))
  (bind _output_get (set `self.CurrentMusicReference` (`|GetArrayItem` (`self.musicreferences`) (`self.IndexSongToPlayLevel`))))
  (`AudioComponent.SetVolumeMultiplier` _output_get 1.0))

(event `ChangeMusicTo`
  (params (IndexOfSongToPlay :type Integer))
  (set `self.IndexSongToPlayLevel` IndexOfSongToPlay)
  (`self.CheckSound`))

(fn `ChangeSound`
  (set `self.CurrentMusicReference` (`|GetArrayItem` (`self.musicreferences`) (`self.IndexSongToPlayLevel`)))
  (`KismetSystemLibrary.K2_SetTimer` null "IncreaseSound" 0.05 true))

(fn `CheckSound`
  (if (== (`self.CurrentMusicReference`) (`|GetArrayItem` (`self.musicreferences`) (`self.IndexSongToPlayLevel`)))
    (set `self.IndexSongToPlayLevel` (- (`self.IndexSongToPlayLevel`) 1)))
  (`KismetSystemLibrary.K2_SetTimer` null "DecreaseSound" 0.05 true))

(fn `DecreaseSound`
  (bind _currentmusicreference (`self.CurrentMusicReference`))
  (bind _volumemultiplier (`AudioComponent.VolumeMultiplier` _currentmusicreference))
  (if (> _volumemultiplier 0.0)
    (`AudioComponent.SetVolumeMultiplier` _currentmusicreference (`KismetMathLibrary.FClamp` (- _volumemultiplier (* (`GameplayStatics.GetWorldDeltaSeconds`) 2.5))))
    (else
      (`self.ChangeSound`)
      (`KismetSystemLibrary.K2_ClearTimer` null "DecreaseSound"))))

(fn `IncreaseSound`
  (bind _currentmusicreference (`self.CurrentMusicReference`))
  (bind _volumemultiplier (`AudioComponent.VolumeMultiplier` _currentmusicreference))
  (if (< _volumemultiplier 1.0)
    (`AudioComponent.SetVolumeMultiplier` _currentmusicreference (`KismetMathLibrary.FClamp` (+ _volumemultiplier (* (`GameplayStatics.GetWorldDeltaSeconds`) 2.5))))
    (else
      (`KismetSystemLibrary.K2_ClearTimer` null "IncreaseSound"))))

(fn `UserConstructionScript`)
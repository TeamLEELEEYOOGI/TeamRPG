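; Health potion pickup that adds a fixed amount of HP when an RPG_Character overlaps its mesh, then destroys itself.
; On BeginPlay it caches player 0's RPGPlayerState, retrying by timer until the cast succeeds.
; Overlap raises that state's HP without clamping and passes current and max HP to the character.
; A fast looping timer, rather than Tick, spins the mesh and bobs it between two heights.
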(event `self.StaticMesh.OnComponentBeginOverlap`
  (params (OverlappedComponent :type "PrimitiveComponent Object Reference") (OtherActor :type "Actor Object Reference") (OtherComp :type "PrimitiveComponent Object Reference") (OtherBodyIndex :type Integer) (bFromSweep :type Boolean) (SweepResult :type "HitResult Structure (by ref)"))
  (bind _as_rpgplayer_state (`self.As RPGPlayer State`))
  (bind _asrpg_character (cast `/Game/Archer/RPG_Character` OtherActor))
  (bind _output_get (set `/Game/JaeSung/GameMode/RPGPlayerState.Hp` (+ 15.0 (`/Game/JaeSung/GameMode/RPGPlayerState.Hp` _as_rpgplayer_state)) _as_rpgplayer_state))
  (`/Game/Archer/RPG_Character.SetHp` _asrpg_character _output_get (`/Game/JaeSung/GameMode/RPGPlayerState.MaxHp` _as_rpgplayer_state))
  (`self.K2_DestroyActor`))

(event `self.ReceiveBeginPlay`
  (`self.BindPlayerState`)
  (`KismetSystemLibrary.K2_SetTimer` null "UpdatePotionMove" 0.01 true))

(fn `BindPlayerState`
  (bind _asrpgplayer_state (cast `/Game/JaeSung/GameMode/RPGPlayerState` (`Controller.PlayerState` (`GameplayStatics.GetPlayerController` 0)))
    (:`then`
      (set `self.As RPGPlayer State` _asrpgplayer_state)
      (`KismetSystemLibrary.K2_ClearTimer` null "BindPlayerState"))
    (:`CastFailed`
      (`KismetSystemLibrary.K2_SetTimer` null "BindPlayerState" 0.1))))

(fn `UpdateMoveUpDown`
  (params (Delta :type "Float (double-precision)"))
  (bind _staticmesh (`self.StaticMesh`))
  (bind _returnvalue (* Delta (`self.Speed`)))
  (bind (_relativelocation_x _relativelocation_y _relativelocation_z) (`KismetMathLibrary.BreakVector` (`SceneComponent.RelativeLocation` (`self.StaticMesh`))))
  (bind (_relativelocation_x_2 _relativelocation_y_2 _relativelocation_z_2) (`KismetMathLibrary.BreakVector` (`SceneComponent.RelativeLocation` (`self.StaticMesh`))))
  (if (`self.IsRight`)
    (`SceneComponent.K2_AddRelativeLocation` _staticmesh (`KismetMathLibrary.MakeVector` 0.0 0.0 _returnvalue) false false)
    (if (> _relativelocation_z 100.0)
      (set `self.IsRight` false))
    (else
      (bind _result (`/Engine/EditorBlueprintResources/StandardMacros.NegateFloat` _returnvalue)
        (:`  `
          (`SceneComponent.K2_AddRelativeLocation` _staticmesh (`KismetMathLibrary.MakeVector` 0.0 0.0 _result) false false)
          (if (< _relativelocation_z_2 50.0)
            (set `self.IsRight` true)))))))

(fn `UpdatePotionMove`
  (`|ExecutionSequence`
    (:`then_0`
      (`self.UpdateRotation` 0.01))
    (:`then_1`
      (`self.UpdateMoveUpDown` 0.01))))

(fn `UpdateRotation`
  (params (Delta :type "Float (double-precision)"))
  (`SceneComponent.K2_AddRelativeRotation` (`self.StaticMesh`) (`KismetMathLibrary.MakeRotator` 0.0 0.0 (* Delta 180.0)) false false))

(fn `UserConstructionScript`)
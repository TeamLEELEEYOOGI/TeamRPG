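; BP_CharacterSelect is an unfinished character-selection Blueprint, apparently for the pre-start stage, built around a SelectCharacter array of character actors.
; InitializeChangeCharacter hides the first array entry when player controller 0 owns this Blueprint, otherwise printing a debug message.
; GetCharacterNo returns the index of the first non-hidden entry.
; ChangeCharacter and BeginPlay are empty, and the nodes that add Archer and BP_Warrior to the array are disconnected.
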(event `self.ReceiveBeginPlay`)

(fn `ChangeCharacter`)

(fn `GetCharacterNo`
  (returns (CharacterNo :type Integer))
  (for (_array_element _array_index) (`self.SelectCharacter`)
    (if (not (`Actor.bHidden` _array_element))
      (return _array_index))))

(fn `InitializeChangeCharacter`
  (if (== (`GameplayStatics.GetPlayerController` 0) (`self.GetOwner`))
    (`self.SetActorHiddenInGame` (`|GetArrayItem` (`self.SelectCharacter`)) true)
    (else
      (`KismetSystemLibrary.PrintString` "조건X" true true (struct :`R` 1.0 :`A` 1.0) 10.0))))

(fn `UserConstructionScript`)
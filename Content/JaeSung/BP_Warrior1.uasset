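; Playable warrior character Blueprint in an RPG, attaching a weapon mesh at BeginPlay and caching its Warrior_AnimBP.
; Input for attack, unequip, evasion and three skills passes through Req/Res event pairs into AnimBP Activate calls.
; The first attack equips and turns on a Niagara effect; evasion requires being equipped and spends stamina via RPGPlayerState.
; Hit and death functions drive AnimBP reactions, with damage recorded on RPGPlayerState.
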(event `self.ReceiveBeginPlay`
  (bind _weapon (`self.Weapon`))
  ;[1 1 1] Initial Skeletal Mesh 합치기, AnimBP 저장
  (`|ExecutionSequence`
    (:`then_0`
      (`SkinnedMeshComponent.SetSkinnedAssetAndUpdate` _weapon "/Game/Warrior/SK_WarriorWeapon.SK_WarriorWeapon" true)
      (`SceneComponent.K2_AttachToComponent` _weapon (`self.Mesh`) "UnEquip_WeaponSocket" "KeepRelative" "KeepRelative" "KeepRelative" true))
    (:`then_1`
      (bind _aswarrior_anim_bp (cast `/Game/Warrior/Warrior_AnimBP` (`SkeletalMeshComponent.GetAnimInstance` (`self.Mesh`))))
      (set `self.As Warrior Anim BP` _aswarrior_anim_bp))))

(event `Key|LeftMouseButton`
  (params (Key :type "Key Structure"))
  ;[1 1 1] Judge Equip
  ; 마우스 왼쪽 클릭시 몽타주 재생 후 Acher_AnimBP의 isEquip을 True로 바꿔준다.
  (:`Pressed`
    (`self.ReqAttack`)))

(event `ReqAttack`
  ;[1 1 1] Judge Equip
  ; 마우스 왼쪽 클릭시 몽타주 재생 후 Acher_AnimBP의 isEquip을 True로 바꿔준다.
  (`self.ResAttack`))

(event `ResAttack`
  ;[1 1 1] Judge Equip
  ; 마우스 왼쪽 클릭시 몽타주 재생 후 Acher_AnimBP의 isEquip을 True로 바꿔준다.
  (`self.SetAttack`))

(event `Key|Tab`
  (params (Key :type "Key Structure"))
  ;[1 1 1] UnEquip
  ; Tab 클릭 시 Archer_AnimBP의 IsEquip을 false로 바꿔준다.
  (:`Pressed`
    (`self.ReqUnEquip`)))

(event `ReqUnEquip`
  ;[1 1 1] UnEquip
  ; Tab 클릭 시 Archer_AnimBP의 IsEquip을 false로 바꿔준다.
  (`self.ResUnEquip`))

(event `ResUnEquip`
  ;[1 1 1] UnEquip
  ; Tab 클릭 시 Archer_AnimBP의 IsEquip을 false로 바꿔준다.
  (if (`self.IsEquip`)
    (set `self.IsEquip` false)
    (`/Game/Warrior/Warrior_AnimBP.ActivateUnEquip` (`self.As Warrior Anim BP`))
    (`ActorComponent.Deactivate` (`self.Niagara1`))))

(event `Key|RightMouseButton`
  (params (Key :type "Key Structure"))
  ;[1 1 1] Evasion 회피
  (:`Pressed`
    (if (`self.IsEquip`)
      (bind _asrpgplayer_state (cast `/Game/JaeSung/GameMode/RPGPlayerState` (`self.PlayerState`)))
      (bind _can (`/Game/JaeSung/GameMode/RPGPlayerState.UpdateStamina` _asrpgplayer_state 10.0 0.0))
      (if _can
        (`self.ReqEvasion`)))))

(event `ReqEvasion`
  ;[1 1 1] Evasion 회피
  (`self.ResEvasion`))

(event `ResEvasion`
  ;[1 1 1] Evasion 회피
  (`/Game/Warrior/Warrior_AnimBP.ActivateEvasion` (`self.As Warrior Anim BP`)))

(event `ReqActivateSkill1`
  ;[1 1 1] warrior skill 1
  (`self.ResActivateSkill1`))

(event `Key|R`
  (params (Key :type "Key Structure"))
  ;[1 1 1] warrior skill 1
  (:`Pressed`
    (`self.ReqActivateSkill1`)))

(event `ResActivateSkill1`
  ;[1 1 1] warrior skill 1
  (`/Game/Warrior/Warrior_AnimBP.ActivateSkill1` (`self.As Warrior Anim BP`)))

(event `ReqActivateSkill2`
  ;[1 1 1] Warrior Skill 2
  (`self.ResActivateSkill2`))

(event `Key|E`
  (params (Key :type "Key Structure"))
  ;[1 1 1] Warrior Skill 2
  (:`Pressed`
    (`self.ReqActivateSkill2`)))

(event `ResActivateSkill2`
  ;[1 1 1] Warrior Skill 2
  (`/Game/Warrior/Warrior_AnimBP.ActivateSkill2` (`self.As Warrior Anim BP`)))

(event `ReqActivateSkill3`
  ;[1 1 1] Warrior Skill 3
  (`self.ResActivateSkill3`))

(event `Key|F`
  (params (Key :type "Key Structure"))
  ;[1 1 1] Warrior Skill 3
  (:`Pressed`
    (`self.ReqActivateSkill3`)))

(event `ResActivateSkill3`
  ;[1 1 1] Warrior Skill 3
  (`/Game/Warrior/Warrior_AnimBP.ActivateSkill3` (`self.As Warrior Anim BP`)))

(fn `SetAttack`
  (`parent.SetAttack`)
  (if (`self.IsEquip`)
    (`/Game/Warrior/Warrior_AnimBP.ActivateAttack` (`self.As Warrior Anim BP`))
    (else
      (set `self.IsEquip` true)
      (`/Game/Warrior/Warrior_AnimBP.ActivateEquip` (`self.As Warrior Anim BP`))
      (`ActorComponent.Activate` (`self.Niagara1`) true))))

(fn `StartDie`
  (`/Game/Warrior/Warrior_AnimBP.ActivateDie` (`self.As Warrior Anim BP`))
  (`parent.StartDie`))

(fn `StartHit`
  (params (DamageKind :type "/Game/JaeSung/GameMode/EnumAttackType Enum" :default "NewEnumerator0") (Damage :type "Float (double-precision)"))
  (bind _aswarrior_anim_bp (cast `/Game/Warrior/Warrior_AnimBP` (`SkeletalMeshComponent.GetAnimInstance` (`self.Mesh`))))
  (`/Game/Warrior/Warrior_AnimBP.ActivateHit` _aswarrior_anim_bp DamageKind)
  (bind _asrpgplayer_state (cast `/Game/JaeSung/GameMode/RPGPlayerState` (`self.PlayerState`)))
  (`/Game/JaeSung/GameMode/RPGPlayerState.AddDamage` _asrpgplayer_state Damage))

(fn `UserConstructionScript`
  (`parent.UserConstructionScript`))
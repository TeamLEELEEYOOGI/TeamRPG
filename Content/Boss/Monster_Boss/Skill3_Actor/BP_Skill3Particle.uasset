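; Projectile actor for a monster boss's third skill: a physics sphere launched forward by an impulse, with optional gravity and a one-second lifetime.
; Construction picks projectile and explosion effects by Level; BeginPlay applies Color and Size to both.
; The first overlap stops the sphere and triggers the explosion, while overlapping RPG_Character actors take fixed damage.
; The position-update function for the projectile effect is never run.
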(event `self.ReceiveBeginPlay`
  (bind _explosion (`self.Explosion`))
  (bind _projectileeffect (`self.ProjectileEffect`))
  (bind _sphere (`self.Sphere`))
  (if (`self.bGravity`)
    (`PrimitiveComponent.SetEnableGravity` _sphere true)
    (else
      (`PrimitiveComponent.SetEnableGravity` _sphere false)))
  (`PrimitiveComponent.AddImpulse` (`self.Sphere`) (* (`self.GetActorForwardVector`) (`self.ImpulsePower`)) "None" true)
  ;[1 1 1] Initialization
  (`FXSystemComponent.SetColorParameter` _projectileeffect "User.Color" (`self.Color`))
  (`FXSystemComponent.SetFloatParameter` _projectileeffect "User.Size" (`self.Size`))
  (`FXSystemComponent.SetColorParameter` _explosion "User.Color" (`self.Color`))
  (`FXSystemComponent.SetFloatParameter` _explosion "User.Size" (`self.Size`))
  (`KismetSystemLibrary.Delay` 1.0)
  (`self.K2_DestroyActor`))

(event `self.ReceiveTick`
  (params (DeltaSeconds :type "Float (single-precision)")))

(event `self.Sphere.OnComponentBeginOverlap`
  (params (OverlappedComponent :type "PrimitiveComponent Object Reference") (OtherActor :type "Actor Object Reference") (OtherComp :type "PrimitiveComponent Object Reference") (OtherBodyIndex :type Integer) (bFromSweep :type Boolean) (SweepResult :type "HitResult Structure (by ref)"))
  (bind _sphere (`self.Sphere`))
  ;[1 1 1] Explode if collision
  (`|ExecutionSequence`
    (:`then_0`
      (`/Engine/EditorBlueprintResources/StandardMacros.DoOnce` false
        (:`Completed`
          (`PrimitiveComponent.SetSimulatePhysics` _sphere false)
          (`PrimitiveComponent.SetCollisionEnabled` _sphere "NoCollision")
          (`ActorComponent.Activate` (`self.Explosion`) true)
          (`KismetSystemLibrary.Delay` 0.5)
          (`ActorComponent.K2_DestroyComponent` (`self.ProjectileEffect`))
          (`KismetSystemLibrary.Delay` 2.0)
          (`self.K2_DestroyActor`))))
    (:`then_1`
      (bind _asrpg_character (cast `/Game/Archer/RPG_Character` OtherActor))
      (`/Engine/EditorBlueprintResources/StandardMacros.IsValid` _asrpg_character
        (:`Is Valid`
          (`/Game/Archer/RPG_Character.StartHit` _asrpg_character "NewEnumerator0" 5.0))))))

(fn `NewFunction_0`
  (bind _projectileeffect (`self.ProjectileEffect`))
  (if (`KismetSystemLibrary.IsValid` _projectileeffect)
    (`FXSystemComponent.SetVectorParameter` _projectileeffect "User.Position" (`SceneComponent.K2_GetComponentLocation` (`self.Sphere`)))))

(fn `UserConstructionScript`
  (bind _explosion (`self.Explosion`))
  (bind _projectileeffect (`self.ProjectileEffect`))
  (switch `int` (`self.Level`)
    (:`Default`
      (`NiagaraComponent.SetAsset` _projectileeffect "/Game/Particle/Stylized_VFX_StPack/Particles/P_Electric_Projectile_03.P_Electric_Projectile_03" true :!label _label)
      (`NiagaraComponent.SetAsset` _explosion "/Game/Particle/Stylized_VFX_StPack/Particles/P_ExplosionEffect_03.P_ExplosionEffect_03" true))
    (:`1`
      (`NiagaraComponent.SetAsset` _projectileeffect "/Game/Particle/Stylized_VFX_StPack/Particles/P_Electric_Projectile_01.P_Electric_Projectile_01" true)
      (`NiagaraComponent.SetAsset` _explosion "/Game/Particle/Stylized_VFX_StPack/Particles/P_ExplosionEffect_01.P_ExplosionEffect_01" true))
    (:`2`
      (`NiagaraComponent.SetAsset` _projectileeffect "/Game/Particle/Stylized_VFX_StPack/Particles/P_Electric_Projectile_02.P_Electric_Projectile_02" true)
      (`NiagaraComponent.SetAsset` _explosion "/Game/Particle/Stylized_VFX_StPack/Particles/P_ExplosionEffect_02.P_ExplosionEffect_02" true))
    (:`3`
      (goto _label))))
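; BP_Arrow_Guided is the Archer's homing arrow projectile, which damages monsters and self-destructs after one second.
; FindNearestMonster, not called within this file, picks the closest BP_Monster overlapping Sphere1 within range and starts a looping AttackMonster timer.
; Each tick of that timer turns Sphere toward the target and offsets it forward without sweep.
; Overlapping a monster applies player-state damage, activates Niagara, stops the timer and destroys the arrow shortly after.
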(event `self.ReceiveBeginPlay`
  (`parent.ReceiveBeginPlay`)
  (`KismetSystemLibrary.Delay` 1.0)
  (`self.K2_DestroyActor`))

(event `self.Sphere.OnComponentBeginOverlap`
  (params (OverlappedComponent :type "PrimitiveComponent Object Reference") (OtherActor :type "Actor Object Reference") (OtherComp :type "PrimitiveComponent Object Reference") (OtherBodyIndex :type Integer) (bFromSweep :type Boolean) (SweepResult :type "HitResult Structure (by ref)"))
  (bind _asbp_monster (cast `/Game/Monster/BP_Monster/Mesh/BP_Monster` OtherActor))
  (`/Engine/EditorBlueprintResources/StandardMacros.IsValid` _asbp_monster
    (:`Is Valid`
      (`/Game/Monster/BP_Monster/Mesh/BP_Monster.ReqUpdateHP` _asbp_monster (`/Game/JaeSung/GameMode/RPGPlayerState.PlayerToMonsterDamage` (`self.As RPGPlayer State`)) (`GameplayStatics.GetPlayerCharacter` 0))
      (`ActorComponent.Activate` (`self.Niagara`) true)
      (`KismetSystemLibrary.K2_ClearTimer` null "AttackMonster")
      (`KismetSystemLibrary.Delay` 0.5)
      (`self.K2_DestroyActor`))))

(fn `ArrowAddWorldOffset`
  (bind _sphere (`self.Sphere`))
  (`SceneComponent.K2_AddWorldOffset` _sphere (* (`SceneComponent.GetForwardVector` _sphere) 50.0) false false))

(fn `AttackMonster`
  (`/Engine/EditorBlueprintResources/StandardMacros.IsValid` (`self.NearestMonster`)
    (:`Is Valid`
      (`self.SetRotationToMonster`)
      (`self.ArrowAddWorldOffset`))))

(fn `FindNearestMonster`
  (bind _overlappingactors (`PrimitiveComponent.GetOverlappingActors` (`self.Sphere1`) "/Game/Monster/BP_Monster/Mesh/BP_Monster.BP_Monster_C"))
  (if (not (<= (`KismetArrayLibrary.Array_Length` _overlappingactors) 0))
    (for _array_element _overlappingactors
      (`/Engine/EditorBlueprintResources/StandardMacros.IsValid` _array_element
        (:`Is Valid`
          (bind _returnvalue (`KismetMathLibrary.VSize` (- (`self.K2_GetActorLocation` _array_element) (`SceneComponent.K2_GetComponentLocation` (`self.Sphere`)))))
          (if (< _returnvalue 3000.0)
            (set `self.Distance` _returnvalue)
            (if (< (`self.Distance`) (`self.NearestDistance`))
              (set `self.NearestDistance` _returnvalue)
              (set `self.NearestMonster` _array_element))))))
    (`/Engine/EditorBlueprintResources/StandardMacros.IsValid` _array_element
      (:`Is Valid`
        (`KismetSystemLibrary.K2_SetTimer` null "AttackMonster" 0.02 true))
      (:`Is Not Valid`
        (`self.K2_DestroyActor`)))))

(fn `SetRotationToMonster`
  (`SceneComponent.K2_SetWorldRotation` (`self.Sphere`) (`KismetMathLibrary.FindLookAtRotation` (`SceneComponent.K2_GetComponentLocation` (`self.SkeletalMesh`)) (`SceneComponent.K2_GetComponentLocation` (`Actor.RootComponent` (`self.NearestMonster`)))) false false))

(fn `UserConstructionScript`
  (`parent.UserConstructionScript`))
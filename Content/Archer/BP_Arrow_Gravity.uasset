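; BP_Arrow_Gravity is an arrow actor that turns into a BP_Portal shortly after launch or upon touching a monster.
; Its Sphere overlap flags contact with a BP_Monster, letting Tick skip its 0.3-second Delay.
; Tick then spawns the portal at the Sphere's X and Y, with a clamped random world Z independent of arrow height, and destroys the arrow.
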(event `self.ReceiveTick`
  (params (DeltaSeconds :type "Float (single-precision)"))
  (bind (_returnvalue_x _returnvalue_y) (`KismetMathLibrary.BreakVector` (`SceneComponent.K2_GetComponentLocation` (`self.Sphere`))))
  (if (not (`self.IsOverlapMonster`))
    (`KismetSystemLibrary.Delay` 0.3))
  (`|SpawnActorFromClass` "/Game/Particle/ArcherParticle/Blueprints/UPDATE_1_2/BP_Portal.BP_Portal_C" (`KismetMathLibrary.MakeTransform` (`KismetMathLibrary.MakeVector` _returnvalue_x _returnvalue_y (`KismetMathLibrary.FClamp` (* (`KismetMathLibrary.RandomFloat`) 300.0) 200.0 300.0))) "Undefined" "OverrideRootScale" null false 5.0 null)
  (`self.K2_DestroyActor`))

(event `self.Sphere.OnComponentBeginOverlap`
  (params (OverlappedComponent :type "PrimitiveComponent Object Reference") (OtherActor :type "Actor Object Reference") (OtherComp :type "PrimitiveComponent Object Reference") (OtherBodyIndex :type Integer) (bFromSweep :type Boolean) (SweepResult :type "HitResult Structure (by ref)"))
  (cast `/Game/Monster/BP_Monster/Mesh/BP_Monster` OtherActor)
  (set `self.IsOverlapMonster` true))

(fn `UserConstructionScript`
  (`parent.UserConstructionScript`))
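; BP_Arrow_Basic is an archer's arrow that damages monsters its sphere overlaps.
; On BeginPlay it runs parent logic and sets a two-second timer calling DestroyArrow, which is not defined here.
; A BP_Monster hit applies damage from the RPG player state, activates Niagara and restores player stamina.
; Other overlaps destroy the arrow after a delay; the monster branch has no destroy call.
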(event `self.ReceiveBeginPlay`
  (`parent.ReceiveBeginPlay`)
  (`KismetSystemLibrary.K2_SetTimer` null "DestroyArrow" 2.0))

(event `self.Sphere.OnComponentBeginOverlap`
  (params (OverlappedComponent :type "PrimitiveComponent Object Reference") (OtherActor :type "Actor Object Reference") (OtherComp :type "PrimitiveComponent Object Reference") (OtherBodyIndex :type Integer) (bFromSweep :type Boolean) (SweepResult :type "HitResult Structure (by ref)"))
  (bind _asbp_monster (cast `/Game/Monster/BP_Monster/Mesh/BP_Monster` OtherActor)
    (:`then`
      (`/Game/Monster/BP_Monster/Mesh/BP_Monster.ReqUpdateHP` _asbp_monster (`/Game/JaeSung/GameMode/RPGPlayerState.PlayerToMonsterDamage` (`self.As RPGPlayer State`)) (`GameplayStatics.GetPlayerCharacter` 0))
      (`ActorComponent.Activate` (`self.Niagara`) true)
      (`/Game/JaeSung/GameMode/RPGPlayerState.UpdateStamina` (`self.As RPGPlayer State`) 0.0 5.0))
    (:`CastFailed`
      (`KismetSystemLibrary.Delay` 2.0)
      (`self.K2_DestroyActor`))))

(fn `UserConstructionScript`
  (`parent.UserConstructionScript`))
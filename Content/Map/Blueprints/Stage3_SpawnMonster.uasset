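; Stage 3 monster spawner Blueprint, a child class that inherits its spawn and respawn behavior from its parent.
; Construction, ReSpawn, SpawnCharacter and SpawnMonster overrides only forward to the parent, and BeginPlay is empty.
; A placeholder-named function, qqqqqqqq, calls SpawnCharacter MonsterSpawnAmount times with the configured pawn class and behavior tree, with no caller in this Blueprint.
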(event `self.ReceiveBeginPlay`)

(fn `qqqqqqqq`
  (for _ (range 1 (+ (`self.MonsterSpawnAmount`) 1))
    (`self.SpawnCharacter` (`self.Pawn Class`) (`self.Behavior Tree`))))

(fn `ReSpawn`
  (`parent.ReSpawn`))

(fn `SpawnCharacter`
  (params (PawnClass :type "Pawn Class Reference") (BehaviorTree :type "BehaviorTree Object Reference"))
  (`parent.SpawnCharacter` PawnClass BehaviorTree))

(fn `SpawnMonster`
  (`parent.SpawnMonster`))

(fn `UserConstructionScript`
  (`parent.UserConstructionScript`))
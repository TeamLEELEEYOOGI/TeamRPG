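; Stage 2 monster spawner, a child Blueprint that inherits its spawn and respawn behavior from a parent class.
; Its construction script, ReSpawn and SpawnCharacter only call the parent versions, and its BeginPlay node is disabled.
; NewFunction_0 loops MonsterSpawnAmount times, calling SpawnCharacter with the PawnClass and BehaviorTree variables; nothing in this file calls it.
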(fn `NewFunction_0`
  (for _ (range 1 (+ (`self.MonsterSpawnAmount`) 1))
    (`self.SpawnCharacter` (`self.Pawn Class`) (`self.Behavior Tree`))))

(fn `ReSpawn`
  (`parent.ReSpawn`))

(fn `SpawnCharacter`
  (params (PawnClass :type "Pawn Class Reference") (BehaviorTree :type "BehaviorTree Object Reference"))
  (`parent.SpawnCharacter` PawnClass BehaviorTree))

(fn `UserConstructionScript`
  (`parent.UserConstructionScript`))
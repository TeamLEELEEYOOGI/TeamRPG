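; BP_MIddleDoubleDoor is a double door that swings open when something overlaps its left door component.
; The overlap starts a fast looping timer on OpenMiddleDoor, which rotates both leaves in opposite yaw directions by Speed and world delta seconds toward 90 degrees.
; The timer clears once the right door reaches its limit, and the file has no closing logic.
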(event `self.Leftdoor.OnComponentBeginOverlap`
  (params (OverlappedComponent :type "PrimitiveComponent Object Reference") (OtherActor :type "Actor Object Reference") (OtherComp :type "PrimitiveComponent Object Reference") (OtherBodyIndex :type Integer) (bFromSweep :type Boolean) (SweepResult :type "HitResult Structure (by ref)"))
  (`KismetSystemLibrary.K2_SetTimer` null "OpenMiddleDoor" 0.01 true))

(fn `OpenMiddleDoor`
  (bind (_relativerotation_roll _relativerotation_pitch _relativerotation_yaw) (`KismetMathLibrary.BreakRotator` (`SceneComponent.RelativeRotation` (`self.Rightdoor`))))
  (bind (_relativerotation_roll_2 _relativerotation_pitch_2 _relativerotation_yaw_2) (`KismetMathLibrary.BreakRotator` (`SceneComponent.RelativeRotation` (`self.Leftdoor`))))
  (`|ExecutionSequence`
    (:`then_0`
      (if (> _relativerotation_yaw_2 -90.0)
        (`SceneComponent.K2_AddRelativeRotation` (`self.Leftdoor`) (`KismetMathLibrary.MakeRotator` 0.0 0.0 (* (* (`self.Speed`) -1.0) (`GameplayStatics.GetWorldDeltaSeconds`))) false false)))
    (:`then_1`
      (if (< _relativerotation_yaw 90.0)
        (`SceneComponent.K2_AddRelativeRotation` (`self.Rightdoor`) (`KismetMathLibrary.MakeRotator` 0.0 0.0 (* (`GameplayStatics.GetWorldDeltaSeconds`) (`self.Speed`))) false false)
        (else
          (`KismetSystemLibrary.K2_ClearTimer` null "OpenMiddleDoor"))))))

(fn `UserConstructionScript`)
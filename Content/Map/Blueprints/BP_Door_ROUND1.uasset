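; Double door actor, named for Round 1, that swings its two leaves open in opposite directions.
; UpdateOpenDoubleDoor starts a fast looping timer on OpenDoubleDoor instead of using Tick; nothing in this Blueprint calls it.
; Each call adds yaw scaled by Speed and world delta seconds until the leaves reach a quarter turn.
; Only the right leaf's limit check clears the timer.
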(fn `OpenDoubleDoor`
  (bind (_relativerotation_roll _relativerotation_pitch _relativerotation_yaw) (`KismetMathLibrary.BreakRotator` (`SceneComponent.RelativeRotation` (`self.RightDoor`))))
  (bind (_relativerotation_roll_2 _relativerotation_pitch_2 _relativerotation_yaw_2) (`KismetMathLibrary.BreakRotator` (`SceneComponent.RelativeRotation` (`self.LeftDoor`))))
  (`|ExecutionSequence`
    (:`then_0`
      (if (> _relativerotation_yaw_2 -90.0)
        (`SceneComponent.K2_AddRelativeRotation` (`self.LeftDoor`) (`KismetMathLibrary.MakeRotator` 0.0 0.0 (* (* (`self.Speed`) -1.0) (`GameplayStatics.GetWorldDeltaSeconds`))) false false)))
    (:`then_1`
      (if (< _relativerotation_yaw 90.0)
        (`SceneComponent.K2_AddRelativeRotation` (`self.RightDoor`) (`KismetMathLibrary.MakeRotator` 0.0 0.0 (* (`GameplayStatics.GetWorldDeltaSeconds`) (`self.Speed`))) false false)
        (else
          (`KismetSystemLibrary.K2_ClearTimer` null "OpenDoubleDoor"))))))

(fn `Update Open Double Door`
  (`KismetSystemLibrary.K2_SetTimer` null "OpenDoubleDoor" 0.01 true))

(fn `UserConstructionScript`)
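; A sliding door Blueprint, BP_Door_ROUND3, that raises its StaticMesh vertically when opened.
; UpdateOpenDoor starts a looping timer on OpenDoor, which moves the mesh up by Speed times world delta seconds.
; OpenDoor clears its own timer once the mesh's relative Z reaches a fixed height.
; Mesh overlap instead starts a looping timer on "MoveTop", a function not defined in this file.
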(event `self.StaticMesh.OnComponentBeginOverlap`
  (params (OverlappedComponent :type "PrimitiveComponent Object Reference") (OtherActor :type "Actor Object Reference") (OtherComp :type "PrimitiveComponent Object Reference") (OtherBodyIndex :type Integer) (bFromSweep :type Boolean) (SweepResult :type "HitResult Structure (by ref)"))
  (`KismetSystemLibrary.K2_SetTimer` null "MoveTop" 0.01 true))

(fn `OpenDoor`
  (bind (_relativelocation_x _relativelocation_y _relativelocation_z) (`KismetMathLibrary.BreakVector` (`SceneComponent.RelativeLocation` (`self.StaticMesh`))))
  (if (< _relativelocation_z 400.0)
    (`SceneComponent.K2_AddRelativeLocation` (`self.StaticMesh`) (`KismetMathLibrary.MakeVector` 0.0 0.0 (* (`GameplayStatics.GetWorldDeltaSeconds`) (`self.Speed`))) false false)
    (else
      (`KismetSystemLibrary.K2_ClearTimer` null "OpenDoor"))))

(fn `UpdateOpenDoor`
  (`KismetSystemLibrary.K2_SetTimer` null "OpenDoor" 0.01 true))

(fn `UserConstructionScript`)
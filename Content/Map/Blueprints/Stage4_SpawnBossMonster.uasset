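; Stage 4 boss spawner Blueprint, a child of a monster spawner class that supplies the spawning logic.
; BeginPlay only sets the pawn class to BP_BossMonster and the behavior tree to Tree_Boss.
; SpawnCharacter, ReSpawn and SpawnMonster just forward to the parent.
; A placeholder-named Rrrrrrrr function spawns MonsterSpawnAmount characters in a loop, with no caller in this Blueprint.
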(event `self.ReceiveBeginPlay`
  (set `self.Pawn Class` "/Game/Boss/Monster_Boss/Char/BP_BossMonster.BP_BossMonster_C")
  (set `self.Behavior Tree` "/Game/Boss/AiControll/Tree_Boss.Tree_Boss"))

(fn `ReSpawn`
  (`parent.ReSpawn`))

(fn `rrrrrrrr`
  (for _ (range 1 (+ (`self.MonsterSpawnAmount`) 1))
    (`self.SpawnCharacter` (`self.Pawn Class`) (`self.Behavior Tree`))))

(fn `SpawnCharacter`
  (params (PawnClass :type "Pawn Class Reference") (BehaviorTree :type "BehaviorTree Object Reference"))
  (`parent.SpawnCharacter` PawnClass BehaviorTree))

(fn `SpawnMonster`
  (`parent.SpawnMonster`))

(fn `UserConstructionScript`
  (`parent.UserConstructionScript`))
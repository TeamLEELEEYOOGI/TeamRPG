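; Stage 1 monster spawner that fills its Bound volume with AI monsters and keeps their population topped up.
; On BeginPlay it spawns the target amount and starts a looping timer that calls ReSpawn to replace any shortfall.
; SpawnCharacter traces downward from above random points in the bounds to place each pawn on WorldStatic geometry, then applies HP and AP to BP_Monster.
; MonsterDie decrements the live count that ReSpawn checks.
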(event `self.ReceiveBeginPlay`
  (`self.SpawnMonster`))

(fn `MonsterDie`
  (returns (Clear :type Boolean))
  (set `self.MonsterCount` (- (`self.MonsterCount`) 1))
  (return true))

(fn `ReSpawn`
  (if (< (`self.MonsterCount`) (`self.MonsterSpawnAmount`))
    (for _ (range 1 (+ (- (`self.MonsterSpawnAmount`) (`self.MonsterCount`)) 1))
      (`self.SpawnCharacter` (`self.Pawn Class`) (`self.Behavior Tree`)))))

(fn `SpawnCharacter`
  (params (PawnClass :type "Pawn Class Reference") (BehaviorTree :type "BehaviorTree Object Reference"))
  (bind (_origin _boxextent) (`KismetSystemLibrary.GetComponentBounds` (`self.bound`)))
  (bind _returnvalue (`KismetMathLibrary.MakeVector` (.x (`KismetMathLibrary.RandomPointInBoundingBox` _origin _boxextent)) (.y (`KismetMathLibrary.RandomPointInBoundingBox` _origin _boxextent)) (+ (.z (`KismetMathLibrary.RandomPointInBoundingBox` _origin _boxextent)) 10000.0)))
  (bind _outhit (`KismetSystemLibrary.LineTraceSingleForObjects` _returnvalue (+ _returnvalue (* (* (`self.GetActorUpVector`) -1.0) 15000.0)) (`|MakeArray` "ObjectTypeQuery1" :!type "EObjectTypeQuery Enum")))
  (bind _returnvalue_2 (`AIBlueprintHelperLibrary.SpawnAIFromClass` PawnClass BehaviorTree (`KismetMathLibrary.MakeVector` (.x (`.Location` (`GameplayStatics.BreakHitResult` _outhit))) (.y (`.Location` (`GameplayStatics.BreakHitResult` _outhit))) (+ (.z (`.Location` (`GameplayStatics.BreakHitResult` _outhit))) 100.0)) (`KismetMathLibrary.MakeRotator` 0.0 0.0 (`KismetMathLibrary.RandomFloat`)) false null))
  (bind _asbp_monster (cast `/Game/Monster/BP_Monster/Mesh/BP_Monster` _returnvalue_2)
    (:`then`
      (`/Game/Monster/BP_Monster/Mesh/BP_Monster.SetHpAp` _asbp_monster (`self.Hp`) (`self.Ap`)))
    (:`CastFailed`
      _))
  (set `self.MonsterCount` (+ (`self.MonsterCount`) 1)))

(fn `SpawnMonster`
  (for _ (range 1 (+ (`self.MonsterSpawnAmount`) 1))
    (`self.SpawnCharacter` (`self.Pawn Class`) (`self.Behavior Tree`)))
  (`KismetSystemLibrary.PrintString` (`KismetStringLibrary.Conv_IntToString` (`self.MonsterCount`)) true true (struct :`R` 1.0 :`B` 0.010379 :`A` 1.0) 30.0)
  (`KismetSystemLibrary.K2_SetTimer` null "ReSpawn" 10.0 true))

(fn `UserConstructionScript`)